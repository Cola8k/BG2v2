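; Game instance Blueprint that manages multiplayer sessions and the end of a match.
; Hosting creates a session, stores the player count and opens M_Arena as a listen server, while joining uses a supplied search result.
; Destroying a session returns to the Lobby level.
; EndGame unpossesses the first player controller and passes the winner to its arena HUD's victory display.
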(event `HostGame`
  (params (PublicConnections :type Integer) (bUseLAN :type Boolean))
  ;[0 0 0] Host
  (`CreateSessionCallbackProxy.CreateSession` (`GameplayStatics.GetPlayerController` 0) PublicConnections bUseLAN
    (:`OnSuccess`
      (set `self.PlayerNumber` PublicConnections)
      (`GameplayStatics.OpenLevel` "M_Arena" true "listen"))
    (:`OnFailure`
      (`KismetSystemLibrary.PrintString` "GameInstance HostGame: Error"))))

(event `JoinGame`
  (params (SessionToJoin :type "BlueprintSessionResult Structure (by ref)"))
  ;[0 0 0] Join
  (`JoinSessionCallbackProxy.JoinSession` (`GameplayStatics.GetPlayerController` 0) SessionToJoin
    (:`then`
      (`KismetSystemLibrary.PrintString` "TryJoin"))
    (:`OnSuccess`
      (`KismetSystemLibrary.PrintString` "Join Success"))
    (:`OnFailure`
      (`KismetSystemLibrary.PrintString` "GameInstance JoinGame: Error"))))

(event `DestroyGame`
  (params (PlayerController :type "PlayerController Object Reference"))
  ;[0 0 0] Destroy
  (`DestroySessionCallbackProxy.DestroySession` PlayerController
    (:`OnSuccess`
      (`GameplayStatics.OpenLevel` "Lobby"))
    (:`OnFailure`
      (`KismetSystemLibrary.PrintString` "GameInstance DestroyGame: Error"))))

(event `EndGame`
  (params (Winner :type "/Game/Team Enum" :default "NewEnumerator0"))
  (bind _returnvalue (`GameplayStatics.GetPlayerController` 0))
  ;[0 0 0] Destroy
  (`KismetSystemLibrary.PrintString` "Hellooooooooooooo" true true (struct :`R` 0.065775 :`B` 1.0 :`A` 1.0) 22.0)
  (`Controller.UnPossess` _returnvalue)
  (bind _asplayer_controller_arena (cast `/Game/Junk/PlayerController_Arena` _returnvalue))
  (`/Game/HUD/HUD_Arena.SetVictory` (`/Game/Junk/PlayerController_Arena.HUD_Ref` _asplayer_controller_arena) Winner))