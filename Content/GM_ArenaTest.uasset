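; Game mode for a two-team arena test that assigns teams, spawns players and decides the winner.
; On login it alternates controllers between Blue and Red, spawning and possessing a Strider at that team's spawner.
; It calls GameStart on all controllers when the player count matches the Game Instance's PlayerNumber.
; PlayerDeath removes players from their team; an emptied team sends the opposing color as victor to dead and surviving players.
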(event `self.ReceiveBeginPlay`
  ;[0 0 0 1 44] Save Game Istance Data
  (bind _asgi_bp (cast `/Game/GI_BP` (`GameplayStatics.GetGameInstance`)))
  (bind _output_get (set `self.GI_Ref` _asgi_bp))
  (set `self.Player Number` (`/Game/GI_BP.PlayerNumber` _output_get))
  (bind _returnvalue (`GameplayStatics.GetActorOfClass` "/Game/RedSpawner.RedSpawner_C"))
  (set `self.R_Spawn` _returnvalue)
  (bind _returnvalue_2 (`GameplayStatics.GetActorOfClass` "/Game/BlueSpawner.BlueSpawner_C"))
  (set `self.B_Spawn` _returnvalue_2))

(event `PlayerDeath`
  (params (Team :type "/Game/Team Enum" :default "NewEnumerator0") (Player :type "/Game/Player/Controller_ArenaTest Object Reference"))
  (bind _deathplayers (`self.DeathPlayers`))
  (`KismetArrayLibrary.Array_Add` (`self.DeathPlayers`) Player)
  (switch `/Game/Team` Team
    (:`NewEnumerator0`
      (`KismetArrayLibrary.Array_RemoveItem` (`self.BlueTeam`) Player)
      (if (== (`KismetArrayLibrary.Array_Length` (`self.BlueTeam`)) 0)
        (`KismetArrayLibrary.Array_Append` _deathplayers (`self.RedTeam`))
        (for _array_element _deathplayers
          (`/Game/Player/Controller_ArenaTest.SetVictory` _array_element "NewEnumerator1"))))
    (:`NewEnumerator1`
      (`KismetArrayLibrary.Array_RemoveItem` (`self.RedTeam`) Player)
      (if (== (`KismetArrayLibrary.Array_Length` (`self.RedTeam`)) 0)
        (`KismetArrayLibrary.Array_Append` _deathplayers (`self.BlueTeam`))
        (for _array_element_2 _deathplayers
          (`/Game/Player/Controller_ArenaTest.SetVictory` _array_element_2 "NewEnumerator0"))))))

(event `self.K2_PostLogin`
  (params (NewPlayer :type "PlayerController Object Reference"))
  (bind _ascontroller_arena_test (cast `/Game/Player/Controller_ArenaTest` NewPlayer))
  (`|ExecutionSequence`
    (:`then_0`
      (`/Engine/EditorBlueprintResources/StandardMacros.FlipFlop`
        (:`A`
          ;[0 0 0 1 44] Assign Team
          (`KismetArrayLibrary.Array_Add` (`self.BlueTeam`) _ascontroller_arena_test)
          ;[0 0 0 1 44] Spawn Player
          (bind _returnvalue (`|SpawnActorFromClass` "/Game/Player/Strider_ArenaTest.Strider_ArenaTest_C" (`self.GetTransform` (`self.B_Spawn`)) "AdjustIfPossibleButAlwaysSpawn" "OverrideRootScale" _ascontroller_arena_test "NewEnumerator0" null))
          ;[0 0 0 1 44] Player_Arena Reacts to Possess Event
          (`Controller.Possess` _ascontroller_arena_test _returnvalue))
        (:`B`
          (`KismetArrayLibrary.Array_Add` (`self.RedTeam`) _ascontroller_arena_test)
          (bind _returnvalue_2 (`|SpawnActorFromClass` "/Game/Player/Strider_ArenaTest.Strider_ArenaTest_C" (`self.GetTransform` (`self.R_Spawn`)) "AdjustIfPossibleButAlwaysSpawn" "OverrideRootScale" _ascontroller_arena_test "NewEnumerator1" null))
          (`Controller.Possess` _ascontroller_arena_test _returnvalue_2)))
      (`/Engine/EditorBlueprintResources/StandardMacros.IncrementInt` (`self.NewVar`)))
    (:`then_1`
      ;[0 0 0 1 44] Game Starts when Players are enough
      (bind _returnvalue_3 (`self.GetNumPlayers`))
      (if (== _returnvalue_3 (`self.Player Number`))
        (for _array_element (`self.BlueTeam`)
          (`/Game/Player/Controller_ArenaTest.GameStart` _array_element))
        (for _array_element_2 (`self.RedTeam`)
          (`/Game/Player/Controller_ArenaTest.GameStart` _array_element_2))))))

(fn `UserConstructionScript`)